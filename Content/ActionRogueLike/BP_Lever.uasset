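; BP_Lever is an interactable lever that triggers a linked SelectedActor.
; Interact tilts HandleMesh to one of two pitches based on IsEnabled, flips that flag, then forwards the Interact interface message to SelectedActor.
; When IsEnabled is true, it also casts SelectedActor to SExplosiveBarrel and calls Explode.
; A failed cast on that branch stops execution before the toggle and the forwarded message.
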(event `SGameplayInterface.Interact`
  (params (InstigatorPawn :type "Pawn Object Reference"))
  (bind _handlemesh (`self.HandleMesh`))
  (if (`self.IsEnabled`)
    (`SceneComponent.K2_SetRelativeRotation` _handlemesh (`KismetMathLibrary.MakeRotator` 0.0 -30.0) false false)
    (bind _assexplosive_barrel (cast `SExplosiveBarrel` (`self.SelectedActor`)))
    (`SExplosiveBarrel.Explode` _assexplosive_barrel)
    (else
      (`SceneComponent.K2_SetRelativeRotation` _handlemesh (`KismetMathLibrary.MakeRotator` 0.0 30.0) false false)))
  (set `self.IsEnabled` (not (`self.IsEnabled`)))
  (message `SGameplayInterface.Interact` (`self.SelectedActor`) InstigatorPawn))

(fn `UserConstructionScript`)